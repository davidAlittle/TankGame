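; Tank Blueprint that handles orbital aim input, with no movement or firing logic in its graphs.
; The AimAzimuth axis yaws the AzGimball component and AimElecation pitches the SpringArm, separating the two rotations, both scaled by frame time and unclamped in the graph.
; An Enableinput0 flag gates both axes and is set true two seconds after BeginPlay.
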(event EventBeginPlay
  (Utilities|FlowControl|Delay 2.0)
  (Variables|Default|Setenableinput_0 true))

(event Collision|EventActorBeginOverlap
  (params (OtherActor :type Actor%20Object%20Reference)))

(event EventTick
  (params (DeltaSeconds :type Float%20%28single-precision%29)))

(event Input|AxisEvents|InputAxisAimAzimuth
  (params (AxisValue :type Float%20%28single-precision%29))
  (if (Variables|Default|Getenableinput_0)
    (Transformation|AddLocalRotation (Variables|Default|GetAzGimball) (Math|Rotator|MakeRotator 0.0 0.0 (* (Utilities|Time|GetWorldDeltaSeconds) AxisValue 1e+02)) false false)))

(event Input|AxisEvents|InputAxisAimElecation
  (params (AxisValue :type Float%20%28single-precision%29))
  (if (Variables|Default|Getenableinput_0)
    (Transformation|AddLocalRotation (Variables|Default|GetSpringArm) (Math|Rotator|MakeRotator 0.0 (* (Utilities|Time|GetWorldDeltaSeconds) AxisValue 1e+02) 0.0) false false)))

(fn ConstructionScript)